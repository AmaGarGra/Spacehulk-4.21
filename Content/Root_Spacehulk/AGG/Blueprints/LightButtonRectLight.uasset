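; LightButtonRectLight is a rect light whose visibility mirrors the on/off state of a linked WallButton.
; On BeginPlay it casts its SwitchActor reference to WallButton and sets the RectLight visibility from IsOn.
; SwitchLight repeats the same update when called, with no caller in this file, and both paths do nothing if the cast fails.
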(event `self.ReceiveBeginPlay`
  (bind _aswall_button (cast `/Game/Root_Spacehulk/AGG/Blueprints/WallButton` (`self.SwitchActor`)))
  (`SceneComponent.SetVisibility` (`self.RectLight`) (`/Game/Root_Spacehulk/AGG/Blueprints/WallButton.IsOn` _aswall_button) false))

(fn `SwitchLight`
  (bind _aswall_button (cast `/Game/Root_Spacehulk/AGG/Blueprints/WallButton` (`self.SwitchActor`)))
  (`SceneComponent.SetVisibility` (`self.RectLight`) (`/Game/Root_Spacehulk/AGG/Blueprints/WallButton.IsOn` _aswall_button) false))

(fn `UserConstructionScript`)